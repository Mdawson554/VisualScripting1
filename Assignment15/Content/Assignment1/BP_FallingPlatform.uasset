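; BP_FallingPlatform is a platform meant to fall when the BP_PlatformingCharacter overlaps it.
; The overlap handler sets a non-looping timer of one frame's delta time for TickFallingPlatform, then calls clear timer with an empty function name.
; TickFallingPlatform offsets the mesh's relative Z by delta time and FallingSpeed, but a zero multiplier cancels the movement.
; A distance check against OriginLocation is left unused.
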(event `OnComponentBeginOverlap_Event`
  (params (OverlappedComponent :type "PrimitiveComponent Object Reference") (OtherActor :type "Actor Object Reference") (OtherComp :type "PrimitiveComponent Object Reference") (OtherBodyIndex :type Integer) (bFromSweep :type Boolean) (SweepResult :type "HitResult Structure (by ref)"))
  (cast `/Game/Variant_Platforming/Blueprints/BP_PlatformingCharacter` OtherActor)
  (`KismetSystemLibrary.K2_SetTimerDelegate` (delegate `TickFallingPlatform`) (`GameplayStatics.GetWorldDeltaSeconds`))
  (`KismetSystemLibrary.K2_ClearTimer` null))

(event `TickFallingPlatform`
  (`SceneComponent.K2_AddRelativeLocation` (`self.PlatformMesh`) (`KismetMathLibrary.MakeVector` 0.0 0.0 (* (* (`GameplayStatics.GetWorldDeltaSeconds`) (`self.falling speed`)) 0.0)) false false))

(fn `UserConstructionScript`)