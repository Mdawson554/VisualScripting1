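; BP_timeCollectible is a collectible that adds time to the platforming character's Timer when that character overlaps its Sphere.
; BeginPlay puts a dynamic material on the Cylinder, and Tick oscillates its MainColor between two colors using a sine of game time.
; The overlap handler only increments the Timer by IncrementTimerAmount, while the construction script and CollectedCoin just call their parent versions.
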(event `self.ReceiveBeginPlay`
  (bind _returnvalue (`PrimitiveComponent.CreateDynamicMaterialInstance` (`self.Cylinder`) 0 (`self.OcelatingMaterial`) "None"))
  (bind _output_get (set `self.MaterialInstance` _returnvalue))
  (`MaterialInstanceDynamic.SetVectorParameterValue` _output_get "MainColor" (struct :`R` 0.004318 :`B` 1.0 :`A` 1.0)))

(event `self.ReceiveTick`
  (params (DeltaSeconds :type "Float (single-precision)"))
  (bind _materialinstance (`self.MaterialInstance`))
  (`MaterialInstanceDynamic.SetVectorParameterValue` _materialinstance (`self.MainColor`) (`self.Value  0`))
  (`MaterialInstanceDynamic.SetVectorParameterValue` _materialinstance (`self.MainColor`) (`KismetMathLibrary.LinearColorLerp` (`self.Value  0`) (`self.Value 1`) (+ (/ (`KismetMathLibrary.Sin` (`KismetSystemLibrary.GetGameTimeInSeconds`)) 2.0) 0.5))))

(event `self.Sphere.OnComponentBeginOverlap`
  (params (OverlappedComponent :type "PrimitiveComponent Object Reference") (OtherActor :type "Actor Object Reference") (OtherComp :type "PrimitiveComponent Object Reference") (OtherBodyIndex :type Integer) (bFromSweep :type Boolean) (SweepResult :type "HitResult Structure (by ref)"))
  (bind _asbp_platforming_character (cast `/Game/Variant_Platforming/Blueprints/BP_PlatformingCharacter` OtherActor))
  (bind _output_get (set `self.As BP Platforming Character` _asbp_platforming_character))
  (set `/Game/Variant_Platforming/Blueprints/BP_PlatformingCharacter.Timer` (+ (`self.IncrementTimerAmount`) (`/Game/Variant_Platforming/Blueprints/BP_PlatformingCharacter.Timer` _output_get)) (`self.As BP Platforming Character`)))

(fn `CollectedCoin`
  (params (Object :type "Object Object Reference"))
  (`parent.CollectedCoin` Object))

(fn `UserConstructionScript`
  (`parent.UserConstructionScript`))