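; BP_SpawnCollectible is a coin spawner actor that spawns a collectible at its own transform when the spot is free.
; On BeginPlay it sets a timer of length Duration, which calls SpawnCoin to spawn the configured Class unless IsCoinSpawned is true.
; The CoinDetector component's begin and end overlaps with BP_Collectible actors set and clear that flag, so occupancy is detected by overlap rather than a stored reference.
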(event `self.ReceiveBeginPlay`
  (`KismetSystemLibrary.K2_SetTimerDelegate` (delegate `SpawnCoin`) (`self.Duration`)))

(event `SpawnCoin`
  (if (not (`self.IsCoinSpawned`))
    (`|SpawnActorFromClass` (`self.Class`) (`self.GetTransform`) "Undefined" "MultiplyWithRoot" null null)))

(event `self.CoinDetector.OnComponentBeginOverlap`
  (params (OverlappedComponent :type "PrimitiveComponent Object Reference") (OtherActor :type "Actor Object Reference") (OtherComp :type "PrimitiveComponent Object Reference") (OtherBodyIndex :type Integer) (bFromSweep :type Boolean) (SweepResult :type "HitResult Structure (by ref)"))
  (cast `/Game/Assignment1/BP_Collectible` OtherActor)
  (set `self.IsCoinSpawned` true))

(event `self.CoinDetector.OnComponentEndOverlap`
  (params (OverlappedComponent :type "PrimitiveComponent Object Reference") (OtherActor :type "Actor Object Reference") (OtherComp :type "PrimitiveComponent Object Reference") (OtherBodyIndex :type Integer))
  (cast `/Game/Assignment1/BP_Collectible` OtherActor)
  (set `self.IsCoinSpawned` false))

(fn `UserConstructionScript`)