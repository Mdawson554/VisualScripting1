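; BP_CoinTrigger is a pressure plate that spawns time collectibles when the platforming character steps on it.
; It spawns one BP_timeCollectible at each SpawnPositions offset from the collider's location and marks the plate deactivated.
; Collider overlaps with collectibles toggle IsTimerCollectibleSpawned, which blocks spawning while true.
; BeginPlay creates a dynamic material instance to set the plate's main color.
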(event `self.ReceiveBeginPlay`
  (bind _returnvalue (`PrimitiveComponent.CreateDynamicMaterialInstance` (`self.PressurePlate`) 0 (`self.pressure plate Material`) "None"))
  (bind _output_get (set `self.MaterialInstance` _returnvalue))
  (`MaterialInstanceDynamic.SetVectorParameterValue` _output_get "MainColor" (`self.Value`)))

(event `self.PressurePlateCollider.OnComponentBeginOverlap`
  (params (OverlappedComponent :type "PrimitiveComponent Object Reference") (OtherActor :type "Actor Object Reference") (OtherComp :type "PrimitiveComponent Object Reference") (OtherBodyIndex :type Integer) (bFromSweep :type Boolean) (SweepResult :type "HitResult Structure (by ref)"))
  (`|ExecutionSequence`
    (:`then_1`
      (cast `/Game/Assignment1/BP_timeCollectible` OtherActor)
      (set `self.IsTimerCollectibleSpawned` true))
    (:`then_2`
      (cast `/Game/Variant_Platforming/Blueprints/BP_PlatformingCharacter` OtherActor)
      (if (not (`self.IsTimerCollectibleSpawned`))
        (`self.PressurePlateCoin`)))))

(event `self.PressurePlateCollider.OnComponentEndOverlap`
  (params (OverlappedComponent :type "PrimitiveComponent Object Reference") (OtherActor :type "Actor Object Reference") (OtherComp :type "PrimitiveComponent Object Reference") (OtherBodyIndex :type Integer))
  (cast `/Game/Assignment1/BP_Collectible` OtherActor)
  (set `self.IsTimerCollectibleSpawned` false))

(event `PressurePlateCoin`
  (for _array_element (`self.SpawnPositions`)
    (`|SpawnActorFromClass` "/Game/Assignment1/BP_timeCollectible.BP_timeCollectible_C" (`KismetMathLibrary.MakeTransform` (+ _array_element (`SceneComponent.K2_GetComponentLocation` (`self.PressurePlateCollider`)))) "Undefined" "MultiplyWithRoot" null null)
    (set `self.IsPressurePlateDeactivated` true)))

(fn `OnPressurePlateActivated`)

(fn `UserConstructionScript`)